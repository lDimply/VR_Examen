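; VR game mode that runs endless enemy waves and creates the wave UI widget.
; Each wave loads its class-to-count enemy pool from DT_FWaveStruct by wave number, falling back to random counts that scale with the wave.
; Random picks from the pool queue on random BP_EnemySpawners up to EnemyMaxCount, with kills pulling replacements.
; Dispatchers broadcast wave and kill changes, and a timer starts the next wave once none remain.
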(event EventBeginPlay
  (CallFunction|GetSpawners)
  ;[1 1 1] Cambiar
  (bind _returnvalue (UserInterface|CreateWidget "/Game/4_UI/WBP_WodeModeUI.WBP_WodeModeUI_C"))
  (Variables|Default|SetIU_Waves _returnvalue)
  (CallFunction|NewWave))

(fn ConstructionScript)

(fn GetSpawners
  ;[0.2526 1 0] Listo
  (bind _outactors (Actor|GetAllActorsOfClass "/Game/2_Blueprints/4_Enemy/Spawner/BP_EnemySpawner.BP_EnemySpawner_C"))
  (Variables|Default|SetBP_EnemySpawners _outactors))

(fn StartWave
  ;[0.1353 1 0] Listo
  (CallFunction|BuildEnemyPool)
  (for _index (range 0 (- (Math|Integer|Min(Integer) (CallFunction|GetPoolSize) (Variables|Default|GetEnemyMaxCount)) 1))
    (bind _enemy (CallFunction|GetEnemyfromPool))
    (Default|AddEnemytoQueue (.OutItem (Utilities|Array|Random (Variables|Default|GetBP_EnemySpawners))) _enemy)))

(fn EndWave
  (Default|CallOnEndWave))

(fn EnterTransition
  (params (TransitionTime :type Float%20%28single-precision%29))
  ;[0 1 0.01606] Listo
  (bind _returnvalue (Utilities|Time|SetTimerbyFunctionName 0 "NewWave" TransitionTime))
  (Variables|Default|SetTransition%20Timer _returnvalue)
  (CallFunction|EndWave))

(fn BuildEnemyPool
  (bind _returnvalue (Utilities|GetDataTableRow "/Game/2_Blueprints/7_Struct/DT_FWaveStruct.DT_FWaveStruct" (Utilities|String|StringToName (Utilities|String|ToString(Integer) (Variables|Default|GetWaveNumber))))
    (:then
      (Variables|Default|SetEnemyPool (Utilities|Struct|BreakS_FWaveStruct _returnvalue))
      (Variables|Default|SetEnemyRemaining (CallFunction|GetPoolSize)))
    (:RowNotFound
      (Utilities|Map|Add (Variables|Default|GetEnemyPool) "/Game/2_Blueprints/4_Enemy/BP_Enemy_Baston.BP_Enemy_Baston_C" (Math|Random|RandomIntegerinRange 10 (* (Variables|Default|GetWaveNumber) 5)))
      (Utilities|Map|Add (Variables|Default|GetEnemyPool) "/Game/2_Blueprints/4_Enemy/BP_Enemy_Chocolate.BP_Enemy_Chocolate_C" (Math|Random|RandomIntegerinRange 5 (* (Variables|Default|GetWaveNumber) 3)))
      (Variables|Default|SetEnemyRemaining (CallFunction|GetPoolSize)))))

(fn GetPoolSize
  (bind _values (Utilities|Map|Values (Variables|Default|GetEnemyPool)))
  (for _array_element _values
    (LocalVariables|SetLocal_Sum (+ _array_element (LocalVariables|GetLocal_Sum))))
  (return (LocalVariables|GetLocal_Sum)))

(fn GetEnemyfromPool
  (bind _keys (Utilities|Map|Keys (Variables|Default|GetEnemyPool)))
  (bind _output_get (LocalVariables|SetLocal_ClassChoise (.OutItem (Utilities|Array|Random _keys))))
  (if (> (- (.Value (Utilities|Map|Find (Variables|Default|GetEnemyPool) _output_get)) 1) 0)
    (Utilities|Map|Add (Variables|Default|GetEnemyPool) (LocalVariables|GetLocal_ClassChoise) (- (.Value (Utilities|Map|Find (Variables|Default|GetEnemyPool) _output_get)) 1))
    (return (LocalVariables|GetLocal_ClassChoise))
    (else
      (Utilities|Map|Remove (Variables|Default|GetEnemyPool) (LocalVariables|GetLocal_ClassChoise))
      (return (LocalVariables|GetLocal_ClassChoise)))))

(fn NewWave
  ;[1 1 1] Ojo
  (Math|Integer|IncrementInt (Variables|Default|GetWaveNumber)
    (:%20%20
      (CallFunction|StartWave)
      (Default|CallOnNewWave (Variables|Default|GetWaveNumber) (Variables|Default|GetEnemyRemaining)))))

(fn OnEnemyDefeated
  ;[0 1 0.03342] Listo
  (bind _result (Math|Integer|DecrementInt (Variables|Default|GetEnemyRemaining))
    (:%20%20
      (Default|CallOnEnemyKilled _result)
      (if (< _result (Variables|Default|GetEnemyMaxCount))
        (if (<= (Variables|Default|GetEnemyRemaining) 0)
          (CallFunction|EnterTransition 5.0))
        (else
          (bind _enemy (CallFunction|GetEnemyfromPool))
          (Default|AddEnemytoQueue (.OutItem (Utilities|Array|Random (Variables|Default|GetBP_EnemySpawners))) _enemy))))))