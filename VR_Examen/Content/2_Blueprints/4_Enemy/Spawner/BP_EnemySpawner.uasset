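; Enemy spawner actor that spawns queued enemy classes at its own location.
; AddEnemyToQueue appends a class and spawns immediately if no BP_Enemy overlaps its Sphere; a looping two-second timer also drains the queue, without that overlap check.
; Each spawned enemy gets an OnDestroyed binding, and the OnEnemyDefeated event forwards defeats to BP_GameModeVR.
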(event Custom|OnEnemyDefeated
  (bind _asbp_game_mode_vr (Utilities|Casting|CastToBP_GameModeVR (Game|GetGameMode)))
  (Default|OnEnemyDefeated _asbp_game_mode_vr))

(event Custom|TryToSpawn
  (CallFunction|SpawnEnemy))

(event EventBeginPlay
  (Utilities|Time|SetTimerbyEvent (delegate Custom|TryToSpawn) 2.0 true))

(fn ConstructionScript)

(fn SpawnEnemy
  (if (Utilities|Array|IsValidIndex (Variables|Default|GetEnemyQueue))
    (bind _returnvalue (Game|SpawnActorfromClass (Utilities|Array|Get(acopy) (Variables|Default|GetEnemyQueue)) (Math|Transform|MakeTransform (Transformation|GetActorLocation) "0, 0, 0" "1.000000,1.000000,1.000000") "AdjustIfPossibleButAlwaysSpawn" "MultiplyWithRoot" 0 0))
    (EventDispatchers|BindEventtoOnDestroyed _returnvalue (EventDispatchers|CreateEvent :!event Custom|OnEnemyDefeated))
    (Utilities|Array|RemoveIndex (Variables|Default|GetEnemyQueue))
    (return true)
    (else
      (return false))))

(fn AddEnemytoQueue
  (params (Enemy%20Class :type BP%20Enemy%20Class%20Reference))
  (Utilities|Array|Add (Variables|Default|GetEnemyQueue) Enemy%20Class)
  (if (not (Utilities|Array|IsValidIndex (Collision|GetOverlappingActors (Variables|Default|GetSphere) "/Game/2_Blueprints/4_Enemy/BP_Enemy.BP_Enemy_C" :!class /Script/Engine.PrimitiveComponent)))
    (CallFunction|SpawnEnemy)))