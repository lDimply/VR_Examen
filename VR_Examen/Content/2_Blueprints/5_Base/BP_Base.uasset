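; BP_Base is the player's base, whose loss of health ends the game in defeat.
; Its Sphere overlap picks out valid actors tagged TurretTarget, casts them to BP_Enemy and calls their ApplyDamage, passing the base itself.
; Tick polls ActualHealth every frame and opens the Derrota level once it falls below zero.
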(event OnComponentBeginOverlap(Sphere)
  (params (OverlappedComponent :type Primitive%20Component%20Object%20Reference) (OtherActor :type Actor%20Object%20Reference) (OtherComp :type Primitive%20Component%20Object%20Reference) (OtherBodyIndex :type Integer) (bFromSweep :type Boolean) (SweepResult :type Hit%20Result%20Structure%20%28by%20ref%29))
  (Utilities|IsValid OtherActor
    (:Is%20Valid
      (if (Actor|ActorHasTag OtherActor "TurretTarget")
        (bind _asbp_enemy (Utilities|Casting|CastToBP_Enemy OtherActor))
        (Default|ApplyDamage _asbp_enemy self)))))

(event EventTick
  (params (DeltaSeconds :type Float%20%28single-precision%29))
  (if (< (Variables|Default|GetactualHealth) 0.0)
    (Game|OpenLevel(byObjectReference) "/Game/vicente/menu/derrota.derrota")))

(fn ConstructionScript)