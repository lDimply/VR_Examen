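; BP_CrankWheel is a grabbable VR hand wheel that sends its turn value to a rotating map Blueprint (BPMapa).
; Grabbing stores the motion controller and starts a looping timer; dropping clears it and requests a timer pause by function name.
; Each tick dots the wheel-to-controller direction with the wheel's right vector, smooths it with FInterpTo, rolls the wheel and messages the map.
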(event OnGrabbed(GrabComponent)
  (params (MotionController :type Motion%20Controller%20Component%20Object%20Reference))
  (Variables|Default|SetMotion%20Controller MotionController)
  (bind _returnvalue (Utilities|Time|SetTimerbyEvent (delegate Custom|Update%20Rotation) 0.02 true)))

(event OnDropped(GrabComponent)
  (Variables|Default|SetMotion%20Controller 0)
  (Class|KismetSystemLibrary|PauseTimer 0 "Update Rotation"))

(event Custom|Update%20Rotation
  (bind _output_get (Variables|Default|SetCurrentValue (Math|Interpolation|FInterpTo (Variables|Default|GetCurrentValue) (* (Math|Rotator|NormalizeAxis (Math|Vector|DotProduct (Math|Rotator|GetRotationXVector (Math|Rotator|FindLookatRotation (Transformation|GetWorldLocation (Variables|Default|GetHandWheel_)) (Transformation|GetWorldLocation (Variables|Default|GetMotion%20Controller)))) (Math|Vector|GetRightVector (Transformation|GetWorldRotation (Variables|Default|GetHandWheel_))))) 1e+01) (Class|KismetSystemLibrary|GetTimerElapsedTimeHandle (stale OnGrabbed(GrabComponent) _returnvalue)) 4.0)))
  (Transformation|AddLocalRotation (Variables|Default|GetHandWheel_) (Math|Rotator|MakeRotator _output_get 0.0 0.0) false false)
  (Class|BPIInteractionValue|CrankWheelValue(Message) (Variables|Default|GetBP_Mapa) (Math|Interpolation|FInterpTo (Variables|Default|GetCurrentValue) (* (Math|Rotator|NormalizeAxis (Math|Vector|DotProduct (Math|Rotator|GetRotationXVector (Math|Rotator|FindLookatRotation (Transformation|GetWorldLocation (Variables|Default|GetHandWheel_)) (Transformation|GetWorldLocation (Variables|Default|GetMotion%20Controller)))) (Math|Vector|GetRightVector (Transformation|GetWorldRotation (Variables|Default|GetHandWheel_))))) 1e+01) (Class|KismetSystemLibrary|GetTimerElapsedTimeHandle (stale OnGrabbed(GrabComponent) _returnvalue)) 4.0)))

(fn ConstructionScript)