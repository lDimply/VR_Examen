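; Automated turret that tracks and shoots actors tagged TurretTarget that enter its detection sphere.
; Entering sets the latest target and starts looping timers for interpolated RojoTop yaw/pitch aiming and fire-rate-paced shooting.
; Shots line-trace toward the target, ignoring the map actor, then spawn socket particles and damage any tagged BP_Enemy hit.
; Any tagged actor leaving clears both stored timers while the target is valid, without retargeting.
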(event OnComponentBeginOverlap(Sphere)
  (params (OverlappedComponent :type Primitive%20Component%20Object%20Reference) (OtherActor :type Actor%20Object%20Reference) (OtherComp :type Primitive%20Component%20Object%20Reference) (OtherBodyIndex :type Integer) (bFromSweep :type Boolean) (SweepResult :type Hit%20Result%20Structure%20%28by%20ref%29))
  ;[1 1 1] Cuando ve al enemigo
  (Utilities|IsValid OtherActor
    (:Is%20Valid
      (if (Actor|ActorHasTag OtherActor "TurretTarget")
        (Variables|Default|SetTarget OtherActor)
        (CallFunction|TrackTarget)))))

(event OnComponentEndOverlap(Sphere)
  (params (OverlappedComponent :type Primitive%20Component%20Object%20Reference) (OtherActor :type Actor%20Object%20Reference) (OtherComp :type Primitive%20Component%20Object%20Reference) (OtherBodyIndex :type Integer))
  (Utilities|IsValid OtherActor
    (:Is%20Valid
      (if (Actor|ActorHasTag OtherActor "TurretTarget")
        (Variables|Default|GetTarget
          (:then
            (Utilities|Time|ClearandInvalidateTimerbyHandle (Variables|Default|GetTimerRef))
            (Utilities|Time|ClearandInvalidateTimerbyHandle (Variables|Default|GetFireTimer)))
          (:else))))))

(event Custom|TrackTarget
  ;[1 1 1] Rotate
  (bind _returnvalue (Utilities|Time|SetTimerbyEvent (delegate Custom|MoveTurret) 0.05 true true))
  (Variables|Default|SetTimerRef _returnvalue)
  (bind _returnvalue_2 (Utilities|Time|SetTimerbyEvent (delegate Custom|ShootTurret) (Variables|Default|GetFireRate) true true))
  (Variables|Default|SetFireTimer _returnvalue_2))

(event Custom|MoveTurret
  (bind _returnvalue (Utilities|Time|GetWorldDeltaSeconds))
  (bind _returnvalue_2 (Transformation|GetActorLocation))
  (bind _target (Variables|Default|GetTarget))
  (bind _rojotop (Variables|Default|GetRojoTop))
  (bind _returnvalue_3 (Transformation|GetActorLocation _target))
  (bind _relativerotation (Variables|/Script/Engine.SceneComponent|GetRelativeRotation _rojotop))
  (bind _returnvalue_4 (Math|Rotator|FindLookatRotation _returnvalue_2 _returnvalue_3))
  (bind _returnvalue_5 (Math|Interpolation|RInterpTo _relativerotation _returnvalue_4 _returnvalue 3e+02))
  ;[1 1 1] Rotate
  (Utilities|IsValid _target
    (:Is%20Valid
      (Transformation|SetRelativeRotation (Variables|Default|GetRojoTop) (Math|Rotator|MakeRotator 0.0 (.pitch _returnvalue_5) (.yaw _returnvalue_5)) false false))))

(event Custom|ShootTurret
  (bind _returnvalue (Actor|GetActorOfClass "/Game/2_Blueprints/8_MapaGiratorio/BP_Mapa.BP_Mapa_C"))
  ;[1 1 1] Rotate
  (bind (_outhit _returnvalue_2) (Collision|LineTraceByChannel (+ (Transformation|GetActorLocation) "0.000000,0.000000,80.000000") (Transformation|GetActorLocation (Variables|Default|GetTarget)) "TraceTypeQuery1" true (Utilities|Array|MakeArray _returnvalue) "ForDuration"))
  (if _returnvalue_2
    (if (Actor|ActorHasTag (.HitActor (Collision|BreakHitResult _outhit)) "TurretTarget")
      (bind _asbp_enemy (Utilities|Casting|CastToBP_Enemy (.HitActor (Collision|BreakHitResult _outhit))))
      (Variables|Default|SetBP%20Enemy _asbp_enemy)
      (Effects|SpawnEmitterAttached "/Game/StarterContent/Particles/P_Fire.P_Fire" (Variables|Default|GetRojoTop) "FireSocket" "0, 0, 0" "0, 0, 0" "0.200000,0.200000,0.200000" "SnapToTarget")
      (bind _returnvalue_3 (Effects|SpawnEmitterAttached "/Game/StarterContent/Particles/P_Steam_Lit.P_Steam_Lit" (Variables|Default|GetRojoTop) "FireSocket"))
      (Effects|Components|ParticleSystem|SetVectorParameter _returnvalue_3 "TargetTest" (Transformation|GetActorLocation (Variables|Default|GetTarget)))
      (Game|Damage|ApplyDamage (Variables|Default|GetBP%20Enemy) (Variables|Default|GetDamage) 0 0))))

(fn ConstructionScript)