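; Base Blueprint for turret placement preview, which finds where a turret can be positioned.
; BeginPlay copies every row of DT_Torretas into the DTTorreta array.
; The PreviewLoop event line-traces forward from the Raycast component with debug drawing, asks any hit actor implementing BPI_TorretaPosition for a transform, and stores it in BuildPreview.
; Nothing in this graph calls PreviewLoop or applies that transform to a visible preview.
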(event Custom|PreviewLoop
  (bind _raycast (Variables|Default|GetRaycast))
  (bind _returnvalue (Transformation|GetWorldTransform _raycast))
  (bind (_outhit _returnvalue_2) (Collision|LineTraceForObjects (.location _returnvalue) (+ (.location _returnvalue) (* (Math|Vector|GetForwardVector (.rotation _returnvalue)) 1.5e+03)) (Variables|Default|GetObject%20Types) false (Variables|Default|GetActors%20to%20Ignore) "ForOneFrame"))
  (if _returnvalue_2
    (if (Utilities|DoesObjectImplementInterface (.HitActor (Collision|BreakHitResult _outhit)) "/Game/2_Blueprints/9_TorretaManager/TorretaPrevisualizacion/BPI/BPI_TorretaPosition.BPI_TorretaPosition_C")
      (bind _transformposition (Class|BPITorretaPosition|Transform(Message) (.HitActor (Collision|BreakHitResult _outhit))))
      (Variables|Default|SetBuildPreview _transformposition))))

(event EventBeginPlay
  (bind _outrownames (DataTable|GetDataTableRowNames "/Game/2_Blueprints/9_TorretaManager/TorretaPrevisualizacion/DataBase/DT_Torretas.DT_Torretas"))
  (for _array_element _outrownames
    (bind _returnvalue (Utilities|GetDataTableRow "/Game/2_Blueprints/9_TorretaManager/TorretaPrevisualizacion/DataBase/DT_Torretas.DT_Torretas" _array_element)
      (:then
        (Utilities|Array|Add (Variables|Default|GetDT_Torreta) _returnvalue)))))

(fn ConstructionScript)