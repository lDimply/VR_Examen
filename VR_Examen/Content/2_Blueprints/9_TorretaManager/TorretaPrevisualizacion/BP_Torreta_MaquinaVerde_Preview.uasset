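; Green machine turret placement preview: a grabbable child Blueprint that shows where a turret will be built and spawns it on release.
; While grabbed, Tick runs PreviewLoop and the green preview loop, which creates a collisionless mesh once and moves it to the BuildPreview transform.
; Dropping spawns the DTTorreta Blueprint for TorretaIndex there and clears the preview mesh, which the next grab restores.
; The generic and red preview loop functions are empty.
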(event OnGrabbed(GrabComponent)
  (params (MotionController :type Motion%20Controller%20Component%20Object%20Reference))
  (Variables|Default|SetisGrabbed? true)
  (Components|StaticMesh|SetStaticMesh (Variables|Default|GetPreview_Mesh_Local) (.StaticMesh (Utilities|Struct|BreakS_Torretas (Utilities|Array|Get(acopy) (Variables|Default|GetDT_Torreta) (Variables|Default|GetTorretaIndex))))))

(event OnDropped(GrabComponent)
  (bind _buildpreview (Variables|Default|GetBuildPreview))
  (Variables|Default|SetisGrabbed? false)
  (Game|SpawnActorfromClass (.Blueprint (Utilities|Struct|BreakS_Torretas (Utilities|Array|Get(acopy) (Variables|Default|GetDT_Torreta) (Variables|Default|GetTorretaIndex)))) (Math|Transform|MakeTransform (.location _buildpreview) (.rotation _buildpreview) "3.000000,3.000000,3.000000") "AdjustIfPossibleButAlwaysSpawn" "MultiplyWithRoot" 0 0)
  (Components|StaticMesh|SetStaticMesh (Variables|Default|GetPreview_Mesh_Local) 0))

(event Custom|Preview%20Mesh%20Loop_Verde
  (bind _buildpreview (Variables|Default|GetBuildPreview))
  (bind _buildpreview_2 (Variables|Default|GetBuildPreview))
  (Utilities|FlowControl|Sequence
    (:then_0
      (Utilities|FlowControl|DoOnce false
        (:Completed
          (bind _returnvalue (AddComponent|AddStaticMeshComponent false (Math|Transform|MakeTransform (.location _buildpreview) (.rotation _buildpreview) (Variables|Default|GetLocalScale))))
          (bind _output_get (Variables|Default|SetPreview_Mesh_Local _returnvalue))
          (Components|StaticMesh|SetStaticMesh _output_get (.StaticMesh (Utilities|Struct|BreakS_Torretas (Utilities|Array|Get(acopy) (Variables|Default|GetDT_Torreta) (Variables|Default|GetTorretaIndex)))))
          (Collision|SetCollisionEnabled (Variables|Default|GetPreview_Mesh_Local) "NoCollision"))))
    (:then_1
      (Transformation|SetWorldTransform (Variables|Default|GetPreview_Mesh_Local) (Math|Transform|MakeTransform (.location _buildpreview_2) (.rotation _buildpreview_2) (Variables|Default|GetLocalScale)) false false))))

(event Custom|Reset%20Build%20Mode
  (bind _buildpreview (Variables|Default|GetBuildPreview))
  (Utilities|FlowControl|DoOnce false) ; enters at Reset
)

(event EventTick
  (params (DeltaSeconds :type Float%20%28single-precision%29))
  (if (Variables|Default|GetisGrabbed?)
    (CallFunction|PreviewLoop)
    (CallFunction|PreviewMeshLoopVerde)))

(fn ConstructionScript
  (|CallParentFunction))

(fn PreviewMeshLoop)

(fn PreviewMeshLoopRoja)