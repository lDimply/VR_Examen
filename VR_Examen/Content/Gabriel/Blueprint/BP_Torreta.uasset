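; BP_Torreta is a turret that looks for BP_EnemigoTorreta pawns, aims its gun head and fires debug line traces without applying damage.
; Every Tick, Distancia runs a sphere overlap to choose the nearest candidate as ObjetivoAtacar.
; With a valid attack target, it stops the idle moves, interpolates the head toward Objetivo with clamped pitch, and traces from the Arrow.
; The overlap loop's else branch starts a fixed idle sweep of chained MoveComponentTo rotations.
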(event Custom|Actualizar%20Rotacion
  (bind _turret_sologun_head (Variables|Default|GetTurret_SoloGun_Head))
  (bind _objetivo_ (Variables|Default|GetObjetivo%20))
  (bind _returnvalue (Transformation|GetWorldLocation _turret_sologun_head))
  (bind _returnvalue_2 (Transformation|GetActorLocation _objetivo_))
  (bind _returnvalue_3 (Math|Rotator|FindLookatRotation _returnvalue _returnvalue_2))
  (bind (_roll _pitch _yaw) (Math|Rotator|BreakRotator _returnvalue_3))
  ;[1 1 1] Actualizar rotacion torreta
  (Transformation|SetWorldRotation (Variables|Default|GetTurret_SoloGun_Head) (Math|Interpolation|RInterpTo (Transformation|GetWorldRotation (Variables|Default|GetTurret_SoloGun_Head)) (Math|Rotator|MakeRotator (.pitch (Class|KismetMathLibrary|NegateRotator (Math|Rotator|MakeRotator 0.0 (Math|Float|ClampAngle _pitch -9e+01 2e+01) 0.0))) 0.0 (- _yaw 9e+01)) (Variables|Default|GetDelta%20Seconds) 5.0) false false))

(event Custom|distancia
  (bind _turret_sologun_head (Variables|Default|GetTurret_SoloGun_Head))
  ;[0.4697 0.6023 1] Logica de estado Activo(apuntando)/Inactivo(rotando)
  (Variables|Default|SetObtenerMejorDistancia (+ (Variables|Default|GetRangoDeDeteccion) 1.0))
  ;;[1 1 1] a que actor va apuntar
  (bind _outactors (Collision|SphereOverlapActors (Transformation|GetActorLocation) (Variables|Default|GetRangoDeDeteccion) (Utilities|Array|MakeArray "ObjectTypeQuery3") "/Game/Gabriel/Blueprint/BP_EnemigoTorreta.BP_EnemigoTorreta_C"))
  (for _array_element _outactors
    (bind _output_get (Variables|Default|SetObjetivoActual _array_element))
    (bind _output_get_2 (Variables|Default|SetObtenerDistanciaActual (Transformation|GetDistanceTo _output_get self)))
    (if (or (< _output_get_2 (Variables|Default|GetObtenerMejorDistancia)) (not (Utilities|IsValid (Variables|Default|GetObtenerMejorObjetivo))))
      (Variables|Default|SetObtenerMejorObjetivo (Variables|Default|GetObjetivoActual))
      (Variables|Default|SetObtenerMejorDistancia (Variables|Default|GetObtenerDistanciaActual))
      (Variables|Default|GetObjetivoAtacar
        (:then
          (Utilities|FlowControl|Sequence
            (:then_0
              (CallFunction|ActualizarRotacion)
              (CallFunction|Disparar))
            (:then_1
              (goto _label_3 Stop))
            (:then_2
              (goto _label_2 Stop))
            (:then_3
              (goto _label_4 Stop))
            (:then_4
              (goto _label Stop))))
        (:else))
      (else
        (Components|MoveComponentTo _turret_sologun_head "0, 0, 0" "0.000000,180.000000,0.000000" false false 1.0 false :!label _label)
        (Components|MoveComponentTo _turret_sologun_head "0, 0, 0" "0.000000,-90.000000,0.000000" false false 1.0 false :!label _label_2)
        (Components|MoveComponentTo _turret_sologun_head "0, 0, 0" "0.000000,0.000000,0.000000" false false 1.0 false :!label _label_3)
        (Components|MoveComponentTo _turret_sologun_head "0, 0, 0" "0.000000,90.000000,0.000000" false false 1.0 false :!label _label_4)
        (CallFunction|RotarAleatoriamente))))
  (Variables|Default|SetObjetivoAtacar (Variables|Default|GetObtenerMejorObjetivo)))

(event Custom|disparar
  (bind _arrow (Variables|Default|GetArrow))
  (bind _returnvalue (Transformation|GetWorldLocation _arrow))
  ;[1 1 1] Disparo por line
  (Collision|LineTraceByChannel _returnvalue (+ _returnvalue (* (Math|Vector|GetForwardVector _arrow) "1500.000000,1500.000000,1500.000000")) "TraceTypeQuery1" false 0 "ForDuration"))

(event Custom|RotarAleatoriamente
  (bind _turret_sologun_head (Variables|Default|GetTurret_SoloGun_Head))
  ;[0.4697 0.6023 1] Logica de estado Activo(apuntando)/Inactivo(rotando)
  (Components|MoveComponentTo _turret_sologun_head "0, 0, 0" "0.000000,180.000000,0.000000" false false 1.0 false)
  (Components|MoveComponentTo _turret_sologun_head "0, 0, 0" "0.000000,-90.000000,0.000000" false false 1.0 false)
  (Components|MoveComponentTo _turret_sologun_head "0, 0, 0" "0.000000,0.000000,0.000000" false false 1.0 false)
  (Components|MoveComponentTo _turret_sologun_head "0, 0, 0" "0.000000,90.000000,0.000000" false false 1.0 false)
  (CallFunction|RotarAleatoriamente))

(event EventBeginPlay)

(event EventTick
  (params (DeltaSeconds :type Float%20%28single-precision%29))
  (Variables|Default|SetDelta%20Seconds DeltaSeconds)
  (CallFunction|Distancia))

(fn ConstructionScript)