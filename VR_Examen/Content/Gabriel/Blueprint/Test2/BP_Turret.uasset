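; BP_Turret is a turret that scans for and aims at pawns tagged TurretTarget.
; A SEARCHING/ATTACKING state runs on Tick; searching sweeps a PoseableMesh bone's yaw back and forth, while the attack event is still empty.
; PawnSensing sightings switch to ATTACKING and snap the bone's world-space yaw toward the target.
; Each sighting restarts a short timer that returns the turret to searching once sightings stop.
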(event OnSeePawn(PawnSensing)
  (params (Pawn :type Pawn%20Object%20Reference))
  (bind _poseablemesh (Variables|Default|GetPoseableMesh))
  (if (Actor|ActorHasTag Pawn "TurretTarget")
    (Variables|Default|SetTarget%20Location (Transformation|GetActorLocation Pawn))
    (Variables|Default|SetTurretState "NewEnumerator1")
    ;[1 1 1] Nombre del hueso
    (bind _returnvalue (Class|PoseableMeshComponent|GetBoneRotationbyName _poseablemesh "Bone" "WorldSpace"))
    (Components|PoseableMesh|SetBoneRotationbyName _poseablemesh "Bone" (Math|Rotator|MakeRotator (.roll _returnvalue) (.pitch _returnvalue) (.yaw (Math|Rotator|FindLookatRotation (Transformation|GetActorLocation) (Variables|Default|GetTarget%20Location)))) "WorldSpace")
    (Utilities|Time|ClearandInvalidateTimerbyHandle (Variables|Default|GetReset%20Turret%20State%20Timer))
    (bind _returnvalue_2 (Utilities|Time|SetTimerbyEvent (delegate Custom|Reset%20Turrent%20State) 1.0))
    (Variables|Default|SetReset%20Turret%20State%20Timer _returnvalue_2)))

(event Custom|Rotate%20Turret
  (bind _returnvalue (Utilities|Time|GetWorldDeltaSeconds))
  (bind _returnvalue_2 (* _returnvalue 5e+01))
  ;[1 1 1] nombre del hueso
  (bind _returnvalue_3 (Class|PoseableMeshComponent|GetBoneRotationbyName (Variables|Default|GetPoseableMesh) "Bone" "ComponentSpace"))
  (Variables|Default|SetShould%20Turret%20Rotate%20Right (or (and (< (.Yaw (Math|Rotator|BreakRotator _returnvalue_3)) 7e+01) (Variables|Default|GetShould%20Turret%20Rotate%20Right)) (and (< (.Yaw (Math|Rotator|BreakRotator _returnvalue_3)) -7e+01) (not (Variables|Default|GetShould%20Turret%20Rotate%20Right)))))
  ;[1 1 1] nombre del hueso
  (Components|PoseableMesh|SetBoneRotationbyName (Variables|Default|GetPoseableMesh) "Bone" (Math|Rotator|MakeRotator (.Roll (Math|Rotator|BreakRotator _returnvalue_3)) (.Pitch (Math|Rotator|BreakRotator _returnvalue_3)) (Math|Float|SelectFloat (+ (.Yaw (Math|Rotator|BreakRotator _returnvalue_3)) _returnvalue_2) (- (.Yaw (Math|Rotator|BreakRotator _returnvalue_3)) _returnvalue_2) (Variables|Default|GetShould%20Turret%20Rotate%20Right))) "ComponentSpace"))

(event Custom|Turret%20Attack)

(event Custom|Reset%20Turrent%20State
  (Variables|Default|SetTurretState "NewEnumerator0"))

(event EventBeginPlay)

(event Collision|EventActorBeginOverlap
  (params (OtherActor :type Actor%20Object%20Reference)))

(event EventTick
  (params (DeltaSeconds :type Float%20%28single-precision%29))
  (switch Utilities|FlowControl|Switch|SwitchonTurret_State (Variables|Default|GetTurretState)
    (:NewEnumerator0
      (CallFunction|RotateTurret))
    (:NewEnumerator1
      (CallFunction|TurretAttack))))

(fn ConstructionScript)